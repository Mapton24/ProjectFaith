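; BP_Eregor is a hero character Blueprint holding an unfinished draft of left/right movement that never runs.
; The disconnected graph compares unwired values to set IsMovingRight and snap the actor between two opposite facings.
; Both directions then share one movement input along the control rotation's yaw-only forward vector, at a constant positive scale.
; The construction script is empty.
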(event Input|EnhancedActionEvents|EnhancedInputActionIA_Move
  (params (ActionValue :type Vector%202D%20Structure) (ElapsedSeconds :type Float%20%28double-precision%29) (TriggeredSeconds :type Float%20%28double-precision%29) (InputAction :type Input%20Action%20Object%20Reference :default "/Game/Input/Actions/IA_Move.IA_Move")))

(fn ConstructionScript)